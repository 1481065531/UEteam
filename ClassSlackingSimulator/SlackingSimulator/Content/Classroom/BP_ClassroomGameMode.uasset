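; Classroom game mode that runs an alert meter for getting caught by a walking teacher while the player looks down.
; Each tick, Alert rises while the character's target pitch is below a downward threshold, at a rate scaled by teacher proximity.
; It decays after a short delay without gains and is logged periodically.
; A full meter latches failure, prints game over and calls FailStart on the character.
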(event `self.ReceiveBeginPlay`
  (bind _outactors (`GameplayStatics.GetAllActorsOfClass` "/Game/Classroom/BP_TeacherWalk.BP_TeacherWalk_C"))
  (set `self.Teacher` (`|GetArrayItem` _outactors)))

(event `self.ReceiveTick`
  (params (DeltaSeconds :type "Float (single-precision)"))
  (bind _returnvalue (`KismetSystemLibrary.GetGameTimeInSeconds`))
  (bind _returnvalue_2 (`GameplayStatics.GetPlayerCharacter` 0))
  (bind _lastalerttime (`self.LastAlertTime`))
  (bind _alert (`self.Alert`))
  (bind _asbp_classroom_character (cast `/Game/Classroom/BP_ClassroomCharacter` _returnvalue_2))
  (if (not (`self.bAlertFailed`))
    (bind _returnvalue_3 (* (* (`KismetMathLibrary.MapRangeClamped` (`KismetMathLibrary.Vector_Distance` (`self.K2_GetActorLocation` _returnvalue_2) (`self.K2_GetActorLocation` (`self.Teacher`))) 120.0 300.0 25.0) DeltaSeconds) (`KismetMathLibrary.SelectFloat` 1.0 0.0 (< (.pitch (`/Game/Classroom/BP_ClassroomCharacter.TargetRot` _asbp_classroom_character)) -20.0))))
    (bind _returnvalue_4 (`KismetMathLibrary.FClamp` (- (+ _alert _returnvalue_3) (* (* (`KismetMathLibrary.SelectFloat` 1.0 0.0 (> (- _returnvalue _lastalerttime) 1.5)) 12.0) DeltaSeconds)) 0.0 100.0))
    (set `self.Alert` _returnvalue_4)
    (if (>= _returnvalue_4 100.0)
      (set `self.bAlertFailed` true)
      (`KismetSystemLibrary.PrintString` "GAME_OVER: ALERT=100" false)
      (bind _asbp_classroom_character_2 (cast `/Game/Classroom/BP_ClassroomCharacter` (`GameplayStatics.GetPlayerCharacter` 0)))
      (`/Game/Classroom/BP_ClassroomCharacter.FailStart` _asbp_classroom_character_2)
      (else
        (set `self.LastAlertTime` (`KismetMathLibrary.SelectFloat` _returnvalue _lastalerttime (> _returnvalue_3 0.0)))
        (if (> (- _returnvalue (`self.LastLogTime`)) 1.0)
          (if (> _alert 0.0)
            (`KismetSystemLibrary.PrintString` (`KismetStringLibrary.Conv_DoubleToString` _alert) false)
            (set `self.LastLogTime` _returnvalue)))))))

(fn `UserConstructionScript`
  (`parent.UserConstructionScript`))