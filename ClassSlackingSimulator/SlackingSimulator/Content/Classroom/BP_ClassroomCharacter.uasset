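; Classroom player character that is fixed in place at an offset from its start and switches between looking down at a phone UI and looking around.
; BeginPlay and Q show the WBP_PhoneUI widget, tilt the view down, enable the cursor and ignore look input.
; Arrow debug keys hide the phone and pick a yaw direction; Tick smoothly interpolates control rotation to that target.
; Space calls TryStop on the phone widget.
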(event Collision|EventActorBeginOverlap
  (params (OtherActor :type Actor%20Object%20Reference)))

(event EventTick
  (params (DeltaSeconds :type Float%20%28single-precision%29))
  (bind _returnvalue (Pawn|GetController))
  (Pawn|SetControlRotation _returnvalue (Math|Interpolation|RInterpTo (Pawn|GetControlRotation _returnvalue :!class /Script/Engine.Controller) (Variables|Default|GetTargetRot) DeltaSeconds 6.0)))

(event EventBeginPlay
  (bind _returnvalue (Game|GetPlayerController 0))
  (Transformation|AddActorWorldOffset "(X=-230.0,Y=450.0,Z=-55.0)")
  (Pawn|Components|CharacterMovement|DisableMovement (Variables|Character|GetCharacterMovement))
  (bind _returnvalue_2 (UserInterface|CreateWidget "/Game/UI/WBP_PhoneUI.WBP_PhoneUI_C"))
  (Variables|Default|SetPhoneWidget _returnvalue_2)
  (UserInterface|Viewport|AddtoViewport (Variables|Default|GetPhoneWidget) 0)
  (Variables|Default|SetTargetRot (Math|Rotator|MakeRotator 0.0 -35.0 -9e+01))
  (Widget|SetVisibility (Variables|Default|GetPhoneWidget) "Visible")
  (Input|SetInputModeGameandUI _returnvalue 0 "DoNotLock" true false)
  (Variables|/Script/Engine.PlayerController|SetbShowMouseCursor _returnvalue true)
  (Input|SetIgnoreLookInput _returnvalue true))

(event Input|KeyboardEvents|DebugKeyQ
  (params (Key :type Key%20Structure) (ActionValue :type Input%20Action%20Value%20Structure))
  (bind _returnvalue (Game|GetPlayerController 0))
  (:Pressed
    (UserInterface|Viewport|AddtoViewport (Variables|Default|GetPhoneWidget) 0)
    (Variables|Default|SetTargetRot (Math|Rotator|MakeRotator 0.0 -35.0 -9e+01))
    (Widget|SetVisibility (Variables|Default|GetPhoneWidget) "Visible")
    (Input|SetInputModeGameandUI _returnvalue 0 "DoNotLock" true false)
    (Variables|/Script/Engine.PlayerController|SetbShowMouseCursor _returnvalue true)
    (Input|SetIgnoreLookInput _returnvalue true)))

(event Input|KeyboardEvents|DebugKeyUp
  (params (Key :type Key%20Structure) (ActionValue :type Input%20Action%20Value%20Structure))
  (:Pressed
    (Variables|Default|SetTargetRot (Math|Rotator|MakeRotator 0.0 0.0 -9e+01))
    (Widget|SetVisibility (Variables|Default|GetPhoneWidget) "Collapsed")))

(event Input|KeyboardEvents|DebugKeyDown
  (params (Key :type Key%20Structure) (ActionValue :type Input%20Action%20Value%20Structure))
  (:Pressed
    (Variables|Default|SetTargetRot (Math|Rotator|MakeRotator 0.0 0.0 9e+01))
    (Widget|SetVisibility (Variables|Default|GetPhoneWidget) "Collapsed")))

(event Input|KeyboardEvents|DebugKeyLeft
  (params (Key :type Key%20Structure) (ActionValue :type Input%20Action%20Value%20Structure))
  (:Pressed
    (Variables|Default|SetTargetRot (Math|Rotator|MakeRotator 0.0 0.0 1.8e+02))
    (Widget|SetVisibility (Variables|Default|GetPhoneWidget) "Collapsed")))

(event Input|KeyboardEvents|DebugKeyRight
  (params (Key :type Key%20Structure) (ActionValue :type Input%20Action%20Value%20Structure))
  (:Pressed
    (Variables|Default|SetTargetRot (Math|Rotator|MakeRotator 0.0 0.0 0.0))
    (Widget|SetVisibility (Variables|Default|GetPhoneWidget) "Collapsed")))

(event Input|KeyboardEvents|DebugKeySpaceBar
  (params (Key :type Key%20Structure) (ActionValue :type Input%20Action%20Value%20Structure))
  (:Pressed
    (bind _aswbp_phone_ui (Utilities|Casting|CastToWBP_PhoneUI (Variables|Default|GetPhoneWidget)))
    (Default|TryStop _aswbp_phone_ui)))

(fn ConstructionScript
  (|CallParentFunction))