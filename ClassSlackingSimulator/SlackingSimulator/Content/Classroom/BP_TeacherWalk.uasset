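; BP_TeacherWalk is a classroom teacher actor that paces back and forth along the world Y axis on its own.
; Each Tick feeds a slow time-based pulse, remapped to -1..1, into AddMovementInput, producing a smooth oscillation without waypoints or AI.
; It also snaps yaw between two opposite facings based on Y velocity.
; Leftover location bound checks and an alternate yaw select are unconnected.
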(event `self.ReceiveTick`
  (params (DeltaSeconds :type "Float (single-precision)"))
  (`self.AddMovementInput` (0.0 1.0 0.0) (- (* (`KismetMathLibrary.MakePulsatingValue` (`KismetSystemLibrary.GetGameTimeInSeconds`) 0.12) 2.0) 1.0))
  (`self.K2_SetActorRotation` (`KismetMathLibrary.MakeRotator` 0.0 0.0 (`KismetMathLibrary.SelectFloat` 0.0 180.0 (< (.y (`self.GetVelocity`)) 0.5)))))

(fn `UserConstructionScript`)